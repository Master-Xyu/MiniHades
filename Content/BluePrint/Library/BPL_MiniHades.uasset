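; BPL_MiniHades is a Blueprint function library for reading and writing the local player's state and action state in MiniHades.
; Each getter and setter takes player controller 0's PlayerState and forwards the call to its matching message function.
; The helpers always target player index 0 and do no validity checks.
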(fn GetSelfPlayerState
  (bind _playerstate (Class|BPIPlayerState|GetPlayerState(Message) (Variables|/Script/Engine.Controller|GetPlayerState (Game|GetPlayerController 0))))
  (return _playerstate))

(fn SetSelfPlayerState
  (params (NewPlayerState :type ST%20Player%20State%20Structure))
  (Class|BPIPlayerState|SetPlayerState(Message) (Variables|/Script/Engine.Controller|GetPlayerState (Game|GetPlayerController 0)) NewPlayerState))

(fn GetSelfPlayerActionState
  (bind _actionstate (Class|BPIPlayerState|GetPlayerActionState(Message) (Variables|/Script/Engine.Controller|GetPlayerState (Game|GetPlayerController 0))))
  (return _actionstate))

(fn SetSelfPlayerActionState
  (params (NewActionState :type E_PlayerActionState%20Enum :default "NewEnumerator0"))
  (Class|BPIPlayerState|SetPlayerActionState(Message) (Variables|/Script/Engine.Controller|GetPlayerState (Game|GetPlayerController 0)) NewActionState))