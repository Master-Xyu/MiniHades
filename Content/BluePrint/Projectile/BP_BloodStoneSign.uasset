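; BP_BloodStoneSign is a pickup actor that restores the player's throw charge on contact.
; Unless spawned as UI, its Sphere simulates physics from BeginPlay.
; When BP_Player overlaps the Box, it writes CurrentThrowCharge to the self player state and destroys itself.
; The new value uses Max, not Min, of current plus one and MaxThrowCharge, so it jumps to at least the maximum.
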(event OnComponentBeginOverlap(Box)
  (params (OverlappedComponent :type Primitive%20Component%20Object%20Reference) (OtherActor :type Actor%20Object%20Reference) (OtherComp :type Primitive%20Component%20Object%20Reference) (OtherBodyIndex :type Integer) (bFromSweep :type Boolean) (SweepResult :type Hit%20Result%20Structure%20%28by%20ref%29))
  (bind _playerstate (CallFunction|GetSelfPlayerState))
  (bind (_currentlife _maxlife _attack _currentthrowcharge _maxthrowcharge) (Utilities|Struct|BreakST_PlayerState _playerstate))
  (Utilities|Casting|CastToBP_Player OtherActor)
  (bind _structout (Utilities|Struct|SetmembersinST_PlayerState _playerstate (Math|Integer|Max(Integer) (+ _currentthrowcharge 1) _maxthrowcharge)))
  (CallFunction|SetSelfPlayerState _structout)
  (Actor|DestroyActor))

(event EventBeginPlay
  (if (not (Variables|Default|GetSpawnAsUI))
    (Physics|SetSimulatePhysics (Variables|Default|GetSphere) true)))

(event Collision|EventActorBeginOverlap
  (params (OtherActor :type Actor%20Object%20Reference)))

(event EventTick
  (params (DeltaSeconds :type Float%20%28single-precision%29)))

(fn ConstructionScript)