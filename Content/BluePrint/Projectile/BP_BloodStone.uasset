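; Blood stone projectile that homes on a Pawn near the cursor, or flies toward a point beyond the cursor.
; BeginPlay picks the target with a debug-drawn sphere trace at the cursor hit.
; Tick re-aims velocity at it, passing a look-at direction to SetVelocityInLocalSpace.
; Overlapping a BP_Enemy calls OnBloodStoneHit and destroys the stone, while timing out without a hit leaves a BP_BloodStoneSign.
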(event OnComponentBeginOverlap(Box)
  (params (OverlappedComponent :type Primitive%20Component%20Object%20Reference) (OtherActor :type Actor%20Object%20Reference) (OtherComp :type Primitive%20Component%20Object%20Reference) (OtherBodyIndex :type Integer) (bFromSweep :type Boolean) (SweepResult :type Hit%20Result%20Structure%20%28by%20ref%29))
  (bind _asbp_enemy (Utilities|Casting|CastToBP_Enemy OtherActor))
  (Variables|Default|SetHitEnemy true)
  (Default|OnBloodStoneHit _asbp_enemy)
  (CallFunction|Die))

(event Custom|Die
  (Actor|DestroyActor)
  (if (not (Variables|Default|GetHitEnemy))
    (Game|SpawnActorfromClass "/Game/BluePrint/Projectile/BP_BloodStoneSign.BP_BloodStoneSign_C" (Transformation|GetActorTransform) "Undefined" "MultiplyWithRoot" 0 0)))

(event EventBeginPlay
  (bind _returnvalue (Game|GetPlayerController 0))
  (bind _array (Utilities|Array|MakeArray "ObjectTypeQuery7"))
  (bind _hitresult (Class|PlayerController|GetHitResultUnderCursorforObjects _returnvalue _array true))
  (bind _location (Collision|BreakHitResult _hitresult))
  (bind _returnvalue_2 (+ _location "0.000000,0.000000,90.000000"))
  (Utilities|FlowControl|Sequence
    (:then_0
      (bind (_outhit _returnvalue_3) (Collision|SphereTraceForObjects _returnvalue_2 _returnvalue_2 2e+02 (Utilities|Array|MakeArray "ObjectTypeQuery3") false 0 "ForDuration"))
      (if _returnvalue_3
        (Variables|Default|SetTraceEnemy (.HitActor (Collision|BreakHitResult _outhit))))
      (Variables|Default|SetTargetLoc (+ (* (Class|KismetMathLibrary|VectorNormal2D (- _returnvalue_2 (Transformation|GetActorLocation)) 0.0001) 3000) _returnvalue_2)))
    (:then_1
      (Utilities|FlowControl|Delay 2.0)
      (CallFunction|Die))))

(event Collision|EventActorBeginOverlap
  (params (OtherActor :type Actor%20Object%20Reference)))

(event EventTick
  (params (DeltaSeconds :type Float%20%28single-precision%29))
  (bind _returnvalue (Transformation|GetActorLocation))
  (Utilities|IsValid (Variables|Default|GetTraceEnemy)
    (:Is%20Valid
      (Game|Components|ProjectileMovement|SetVelocityinLocalSpace (Variables|Default|GetProjectileMovement) (* (Math|Rotator|GetRotationXVector (Math|Rotator|FindLookatRotation _returnvalue (Math|Interpolation|VInterpTo _returnvalue (Transformation|GetActorLocation (Variables|Default|GetTraceEnemy)) DeltaSeconds 0.01))) (Variables|Default|GetSpeed))))
    (:Is%20Not%20Valid
      (Game|Components|ProjectileMovement|SetVelocityinLocalSpace (Variables|Default|GetProjectileMovement) (* (Math|Rotator|GetRotationXVector (Math|Rotator|FindLookatRotation _returnvalue (Math|Interpolation|VInterpTo _returnvalue (Variables|Default|GetTargetLoc) DeltaSeconds 0.01))) (Variables|Default|GetSpeed))))))

(fn ConstructionScript)