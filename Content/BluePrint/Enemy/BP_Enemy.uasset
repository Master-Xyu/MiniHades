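; Enemy Blueprint that tracks life and accumulates blood stone hits, dying when damage brings its life to zero.
; Each blood stone hit increments a charge in EnemyState, attaches a BP_BloodStoneSign above the enemy and restarts a drop timer.
; When the timer expires, the signs detach, scatter downward, gain physics after a brief delay, and the charge resets.
; On death, held signs drop with physics before the actor is destroyed.
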(event Custom|OnBloodStoneHit
  (bind _returnvalue (Transformation|GetActorTransform))
  (Utilities|Time|ClearandInvalidateTimerbyHandle (Variables|Default|GetBloodStoneTimer))
  (bind _structout (Utilities|Struct|SetmembersinST_PlayerState (Variables|Default|GetEnemyState) (+ (.CurrentThrowCharge (Utilities|Struct|BreakST_PlayerState (Variables|Default|GetEnemyState))) 1)))
  (Variables|Default|SetEnemyState _structout)
  (bind _returnvalue_2 (Utilities|Time|SetTimerbyEvent (delegate Custom|BloodStoneDrop) 5.0))
  (Variables|Default|SetBloodStoneTimer _returnvalue_2)
  (bind _returnvalue_3 (Game|SpawnActorfromClass "/Game/BluePrint/Projectile/BP_BloodStoneSign.BP_BloodStoneSign_C" (Math|Transform|MakeTransform (+ (.location _returnvalue) "0.000000,0.000000,150.000000") (.rotation _returnvalue) (.scale _returnvalue)) "Undefined" "MultiplyWithRoot" 0 true 0))
  (Transformation|AttachActorToActor _returnvalue_3 self "None" "KeepWorld" "KeepWorld" "KeepWorld" false)
  (Utilities|Array|Add (Variables|Default|GetBloodStoneSigns) _returnvalue_3))

(event Custom|BloodStoneDrop
  (bind _bloodstonesigns (Variables|Default|GetBloodStoneSigns))
  (for _array_element (Variables|Default|GetBloodStoneSigns)
    (Transformation|DetachFromActor _array_element "KeepWorld" "KeepWorld" "KeepWorld")
    (Transformation|SetActorLocation _array_element (+ (Transformation|GetActorLocation _array_element) "0.000000,0.000000,-150.000000" (* (Math|Random|RandomUnitVector) (Math|Random|RandomFloatinRange 2e+01 4e+01))) false false))
  (Utilities|Time|ClearandInvalidateTimerbyHandle (Variables|Default|GetBloodStoneTimer))
  (bind _structout (Utilities|Struct|SetmembersinST_PlayerState (Variables|Default|GetEnemyState) 0))
  (Variables|Default|SetEnemyState _structout)
  (Utilities|FlowControl|Delay 0.036)
  (for _array_element_2 _bloodstonesigns
    (Physics|SetSimulatePhysics (Variables|/Game/BluePrint/Projectile/BP_BloodStoneSign.BP_BloodStoneSign_C|GetSphere _array_element_2) true))
  (Utilities|Array|Clear _bloodstonesigns))

(event EventBeginPlay)

(event Collision|EventActorBeginOverlap
  (params (OtherActor :type Actor%20Object%20Reference)))

(event EventTick
  (params (DeltaSeconds :type Float%20%28single-precision%29)))

(event Game|Damage|EventAnyDamage
  (params (Damage :type Float%20%28single-precision%29) (DamageType :type Damage%20Type%20Object%20Reference) (InstigatedBy :type Controller%20Object%20Reference) (DamageCauser :type Actor%20Object%20Reference))
  (bind _structout (Utilities|Struct|SetmembersinST_PlayerState (Variables|Default|GetEnemyState) (Math|Float|Max(Float) (- (.CurrentLife (Utilities|Struct|BreakST_PlayerState (Variables|Default|GetEnemyState))) Damage) 0.0)))
  (bind _output_get (Variables|Default|SetEnemyState _structout))
  (if (<= (.CurrentLife (Utilities|Struct|BreakST_PlayerState _output_get)) 0.0)
    (CallFunction|OnEnemyDie)))

(fn ConstructionScript)

(fn OnEnemyDie
  (for _array_element (Variables|Default|GetBloodStoneSigns)
    (Transformation|DetachFromActor _array_element "KeepWorld" "KeepWorld" "KeepWorld")
    (Transformation|SetActorLocation _array_element (+ (Transformation|GetActorLocation _array_element) "0.000000,0.000000,-200.000000") false false)
    (Physics|SetSimulatePhysics (Variables|/Game/BluePrint/Projectile/BP_BloodStoneSign.BP_BloodStoneSign_C|GetSphere _array_element) true))
  (Actor|DestroyActor))