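; Player controller that sets up the game camera and provides combat damage and blood stone helpers.
; On BeginPlay it spawns BP_Camera linked to the pawn, makes it the view target and enables game-and-UI input.
; CalcDmg returns player-state Attack, multiplied for backstabs when enemy-to-player world yaw is at or beyond ±120°, ignoring enemy facing.
; BloodStoneOut spawns a BP_BloodStone at the pawn's location.
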(event EventBeginPlay
  (bind _returnvalue (Game|Player|GetPlayerPawn 0))
  (bind _returnvalue_2 (Game|SpawnActorfromClass "/Game/BluePrint/BP_Camera.BP_Camera_C" (Transformation|GetActorTransform _returnvalue) "Undefined" "MultiplyWithRoot" 0 _returnvalue 0))
  (Game|Player|SetViewTargetwithBlend _returnvalue_2 0.0 "VTBlend_Linear" 0.0 false)
  (Input|SetInputModeGameandUI self 0 "DoNotLock" true false))

(event EventTick
  (params (DeltaSeconds :type Float%20%28single-precision%29)))

(fn ConstructionScript)

(fn CalcDmg
  (params (Enemy :type Actor%20Object%20Reference))
  (bind _asbp_enemy (Utilities|Casting|CastToBP_Enemy Enemy))
  (bind _playerstate (Class|BPIPlayerState|GetPlayerState(Message) (Variables|GetPlayerState)))
  (if (or (>= (.yaw (Math|Rotator|FindLookatRotation (Transformation|GetActorLocation _asbp_enemy) (Transformation|GetActorLocation (Game|Player|GetPlayerPawn 0)))) 1.2e+02) (<= (.yaw (Math|Rotator|FindLookatRotation (Transformation|GetActorLocation _asbp_enemy) (Transformation|GetActorLocation (Game|Player|GetPlayerPawn 0)))) -1.2e+02))
    (return (* (.Attack (Utilities|Struct|BreakST_PlayerState _playerstate)) (.BackStubMulti (Utilities|Struct|BreakST_PlayerState _playerstate))))
    (else
      (return (.Attack (Utilities|Struct|BreakST_PlayerState _playerstate))))))

(fn BloodStoneOut
  (Game|SpawnActorfromClass "/Game/BluePrint/Projectile/BP_BloodStone.BP_BloodStone_C" (Math|Transform|MakeTransform (.location (Transformation|GetActorTransform (Game|Player|GetPlayerPawn 0))) "0, 0, 0" "1.000000,1.000000,1.000000") "AlwaysSpawn" "MultiplyWithRoot" 0 0))